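; PlanetC is a planet actor that pulls spaceships toward it and ends the game when hit.
; Each tick, while a SpaceshipActorTest is within range of its Sphere, it adds a fixed velocity toward the planet to every ship's capsule.
; First range entry starts a looping GravTime counter, cleared when out of range, though the pull ignores it.
; A hit sets GameOver on the GameManager, pauses and shows the GameLose widget.
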(event `self.ReceiveHit`
  (params (MyComp :type "PrimitiveComponent Object Reference") (Other :type "Actor Object Reference") (OtherComp :type "PrimitiveComponent Object Reference") (bSelfMoved :type Boolean) (HitLocation :type "Vector Structure") (HitNormal :type "Vector Structure") (NormalImpulse :type "Vector Structure") (Hit :type "HitResult Structure (by ref)"))
  (bind _asgame_manager (cast `/Game/Blueprints/GameManager` (`GameplayStatics.GetGameInstance`)))
  (set `/Game/Blueprints/GameManager.GameOver` true _asgame_manager)
  (`GameplayStatics.SetGamePaused` true)
  (bind _returnvalue (`|CreateWidget` "/Game/Blueprints/UI/GameLose.GameLose_C" (`GameplayStatics.GetPlayerController` 0)))
  (`UserWidget.AddToViewport` _returnvalue 0))

(event `self.ReceiveTick`
  (params (DeltaSeconds :type "Float (single-precision)"))
  (bind _outactors (`GameplayStatics.GetAllActorsOfClass` "/Game/Blueprints/Spaceship-Actor-Test.Spaceship-Actor-Test_C"))
  (for _array_element _outactors
    (if (< (`KismetMathLibrary.Vector_Distance` (`SceneComponent.K2_GetComponentLocation` (`Actor.RootComponent` _array_element)) (`SceneComponent.K2_GetComponentLocation` (`self.Sphere`))) 15000.0)
      (if (`self.EnteredGrav`)
        (bind _outactors_2 (`GameplayStatics.GetAllActorsOfClass` "/Game/Blueprints/Spaceship-Actor-Test.Spaceship-Actor-Test_C"))
        (for _array_element_2 _outactors_2
          (`PrimitiveComponent.SetPhysicsLinearVelocity` (`Character.CapsuleComponent` _array_element_2) (* (`KismetMathLibrary.GetForwardVector` (`KismetMathLibrary.FindLookAtRotation` (`SceneComponent.K2_GetComponentLocation` (`Actor.RootComponent` _array_element_2)) (`SceneComponent.K2_GetComponentLocation` (`self.Sphere`)))) 50.0) true "None"))
        (else
          (`self.InGravityRange`)
          (set `self.EnteredGrav` true)))
      (else
        (`self.NotInGravityRange`)))))

(event `InGravityRange`
  (bind _returnvalue (`KismetSystemLibrary.K2_SetTimerDelegate` (delegate `AccelerateGrav`) 1.0 true)))

(event `NotInGravityRange`
  (`KismetSystemLibrary.K2_ClearAndInvalidateTimerHandle` (stale `InGravityRange` _returnvalue))
  (set `self.GravTime` 0))

(event `AccelerateGrav`
  (set `self.GravTime` (+ (`self.GravTime`) 1)))

(fn `UserConstructionScript`)