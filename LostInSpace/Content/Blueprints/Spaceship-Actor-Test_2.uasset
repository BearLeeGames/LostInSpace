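; Test spaceship pawn with character movement components, steered by yaw input and held on the Z=0 plane.
; BeginPlay and both press and release of Acceleration add forward physics velocity to the capsule, with a larger boost on press.
; A second Acceleration handler raises and lowers CharacterMovement's MaxFlySpeed.
; Tick teleports capsule and mesh to the capsule's XY at zero height; AddMovementInput movement nodes are left unconnected.
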(event `InputAction|Acceleration`
  (params (Key :type "Key Structure"))
  (bind _capsulecomponent (`self.CapsuleComponent`))
  (:`Pressed`
    (`PrimitiveComponent.SetPhysicsLinearVelocity` _capsulecomponent (* (`self.GetActorForwardVector`) 0) true "None")
    (`PrimitiveComponent.SetPhysicsLinearVelocity` _capsulecomponent (* (`self.GetActorForwardVector`) 4000) true "None"))
  (:`Released`
    (`PrimitiveComponent.SetPhysicsLinearVelocity` _capsulecomponent (* (`self.GetActorForwardVector`) 0) true "None" :!label _label)
    (`PrimitiveComponent.SetPhysicsLinearVelocity` _capsulecomponent (* (`self.GetActorForwardVector`) 3300) true "None")))

(event `self.ReceiveBeginPlay`
  (goto _label))

(event `InputAxis|MoveRight`
  (params (AxisValue :type "Float (single-precision)"))
  (`self.AddControllerYawInput` AxisValue))

(event `self.ReceiveTick`
  (params (DeltaSeconds :type "Float (single-precision)"))
  (bind _capsulecomponent (`self.CapsuleComponent`))
  (bind (_returnvalue_x _returnvalue_y) (`KismetMathLibrary.BreakVector` (`SceneComponent.K2_GetComponentLocation` _capsulecomponent)))
  (`SceneComponent.K2_SetWorldLocation` _capsulecomponent (`KismetMathLibrary.MakeVector` _returnvalue_x _returnvalue_y 0.0) false true)
  (`SceneComponent.K2_SetWorldLocation` (`self.StaticMesh`) (`KismetMathLibrary.MakeVector` _returnvalue_x _returnvalue_y 0.0) false true))

(event `InputAction|Acceleration`
  (params (Key :type "Key Structure"))
  (bind _charactermovement (`self.CharacterMovement`))
  ;[1 1 1] Acceleration
  (:`Pressed`
    (set `CharacterMovementComponent.MaxFlySpeed` 2000.0 _charactermovement))
  (:`Released`
    (set `CharacterMovementComponent.MaxFlySpeed` 1200.0 _charactermovement)))

(fn `UserConstructionScript`)