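; Planet actor that acts as a gravity source, pulling GravityAffected actors toward its Sphere.
; Every tick it finds all GravityAffected actors and adds velocity to each one's Cube along the look-at direction to the Sphere.
; The pull is a fixed amount per frame, with no distance falloff or delta-time scaling, so it depends on frame rate.
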(event `self.ReceiveTick`
  (params (DeltaSeconds :type "Float (single-precision)"))
  (bind _outactors (`GameplayStatics.GetAllActorsOfClass` "/Game/Blueprints/GravityAffected.GravityAffected_C"))
  (for _array_element _outactors
    (`PrimitiveComponent.SetPhysicsLinearVelocity` (`/Game/Blueprints/GravityAffected.Cube` _array_element) (* (`KismetMathLibrary.GetForwardVector` (`KismetMathLibrary.FindLookAtRotation` (`SceneComponent.K2_GetComponentLocation` (`/Game/Blueprints/GravityAffected.Cube` _array_element)) (`SceneComponent.K2_GetComponentLocation` (`self.Sphere`)))) 9.8) true "None")))

(fn `UserConstructionScript`)