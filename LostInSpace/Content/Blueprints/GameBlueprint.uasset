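; GameBlueprint watches for the end of a game and restarts it on either a loss or a win.
; Every Tick it polls the GameOver and Win flags on the GameManager game instance, checking GameOver first.
; When either flag is set, it calls RestartGame on the GameMode, without clearing the flag itself.
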(event `self.ReceiveTick`
  (params (DeltaSeconds :type "Float (single-precision)"))
  (bind _asgame_manager (cast `/Game/Blueprints/GameManager` (`GameplayStatics.GetGameInstance`)))
  (if (`/Game/Blueprints/GameManager.GameOver` _asgame_manager)
    (bind _asgame_mode (cast `GameMode` (`GameplayStatics.GetGameMode`)))
    (`GameMode.RestartGame` _asgame_mode)
    (else
      (bind _asgame_manager_2 (cast `/Game/Blueprints/GameManager` (`GameplayStatics.GetGameInstance`)))
      (if (`/Game/Blueprints/GameManager.Win` _asgame_manager_2)
        (bind _asgame_mode_2 (cast `GameMode` (`GameplayStatics.GetGameMode`)))
        (`GameMode.RestartGame` _asgame_mode_2)))))

(fn `UserConstructionScript`)