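; Player-controlled spaceship Character that flies forward, steers by yaw from the MoveRight axis and responds to an Acceleration input.
; BeginPlay gives the capsule a forward physics velocity kick; pressing Acceleration adds a stronger one, and releasing adds the BeginPlay kick again rather than resetting speed.
; The same input also switches CharacterMovement's max fly speed between boosted and normal.
; AddMovementInput nodes are left unwired and never run.
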(event `InputAction|Acceleration`
  (params (Key :type "Key Structure"))
  (:`Pressed`
    (`PrimitiveComponent.SetPhysicsLinearVelocity` (`self.CapsuleComponent`) (* (`self.GetActorForwardVector`) 4000) true "None"))
  (:`Released`
    (`PrimitiveComponent.SetPhysicsLinearVelocity` (`self.CapsuleComponent`) (* (`self.GetActorForwardVector`) 3300) true "None" :!label _label)))

(event `self.ReceiveBeginPlay`
  (goto _label))

(event `InputAxis|MoveRight`
  (params (AxisValue :type "Float (single-precision)"))
  (`self.AddControllerYawInput` AxisValue))

(event `InputAction|Acceleration`
  (params (Key :type "Key Structure"))
  (bind _charactermovement (`self.CharacterMovement`))
  ;[1 1 1] Acceleration
  (:`Pressed`
    (set `CharacterMovementComponent.MaxFlySpeed` 2000.0 _charactermovement))
  (:`Released`
    (set `CharacterMovementComponent.MaxFlySpeed` 1200.0 _charactermovement)))

(fn `UserConstructionScript`)